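; BP_ChefCharacter is the chef character, which interacts with workstations.
; On BeginPlay it adds the IMC_Chef Enhanced Input mapping context to its player controller.
; A hard-bound E key runs a debug-drawn sphere trace from the capsule along world +X, independent of facing.
; If the hit actor is a WorkStationBase, it calls Interact on it, passing itself.
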(event `self.ReceiveBeginPlay`
  (bind _asplayer_controller (cast `PlayerController` (`self.GetController` self)))
  (`EnhancedInputSubsystemInterface.AddMappingContext` (pcsubsystem `EnhancedInputLocalPlayerSubsystem` _asplayer_controller) "/Game/Input/IMC_Chef.IMC_Chef" 0 (struct)))

(event `Key|E`
  (params (Key :type "Key Structure"))
  (bind _returnvalue (`SceneComponent.K2_GetComponentLocation` (`self.CapsuleComponent`)))
  (:`Pressed`
    (bind _outhit (`KismetSystemLibrary.SphereTraceSingle` :`Start` _returnvalue :`End` (+ _returnvalue (100.0 0.0 0.0)) :`Radius` 50.0 :`TraceChannel` "TraceTypeQuery1" :`DrawDebugType` "ForOneFrame"))
    (bind _aswork_station_base (cast `WorkStationBase` (`.HitActor` (`GameplayStatics.BreakHitResult` _outhit))))
    (`WorkStationBase.Interact` _aswork_station_base self)))

(fn `UserConstructionScript`)