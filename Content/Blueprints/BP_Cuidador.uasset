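; BP_Cuidador is the caretaker actor, with a single E key action for interacting and releasing a held object.
; If ObjetoAgarrado is valid, E re-enables physics on its static mesh and calls DetachFromActor on the caretaker itself, without clearing the reference.
; Otherwise, a short forward Visibility line trace sends the Interactuar interface message to the hit actor, passing itself.
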(event `Key|E`
  (params (Key :type "Key Structure"))
  (bind _returnvalue (`self.K2_GetActorLocation`))
  (:`Pressed`
    (`/Engine/EditorBlueprintResources/StandardMacros.IsValid` (`self.ObjetoAgarrado`)
      (:`Is Valid`
        (`PrimitiveComponent.SetSimulatePhysics` (`self.GetComponentByClass` (`self.ObjetoAgarrado`) "/Script/Engine.StaticMeshComponent") true)
        (`self.K2_DetachFromActor` "KeepWorld"))
      (:`Is Not Valid`
        (bind _outhit (`KismetSystemLibrary.LineTraceSingle` _returnvalue (+ (* (`self.GetActorForwardVector`) 200.0) _returnvalue) "TraceTypeQuery1"))
        (message `/Game/Blueprints/BPI_Interaccion.Interactuar` (`.HitActor` (`GameplayStatics.BreakHitResult` _outhit)) self)))))

(fn `UserConstructionScript`)