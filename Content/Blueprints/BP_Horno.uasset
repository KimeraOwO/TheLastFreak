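; BP_Horno is an interactable oven that turns raw meat held by a BP_Cuidador into cooked meat.
; On Interactuar, if the held object is BP_Carne_Cruda, a fixed delay runs before that meat is destroyed and BP_Carne_Cocida spawns at PuntoDeEntrega.
; The spawned meat is stored in CarneEnHorno; while valid, the next interaction is forwarded to it and the reference is cleared.
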(event `/Game/Blueprints/BPI_Interaccion.Interactuar`
  (params (Interactor :type "Actor Object Reference"))
  (bind _carneenhorno (`self.CarneEnHorno`))
  (bind _asbp_cuidador (cast `/Game/Blueprints/BP_Cuidador` Interactor))
  (`parent.Interactuar` null)
  (`/Engine/EditorBlueprintResources/StandardMacros.IsValid` _carneenhorno
    (:`Is Valid`
      (message `/Game/Blueprints/BPI_Interaccion.Interactuar` _carneenhorno _asbp_cuidador)
      (set `self.CarneEnHorno` null))
    (:`Is Not Valid`
      (bind _asbp_carne_cruda (cast `/Game/Blueprints/BP_Carne_Cruda` (`/Game/Blueprints/BP_Cuidador.ObjetoAgarrado` _asbp_cuidador)))
      (`KismetSystemLibrary.Delay` 5.0)
      (`self.K2_DestroyActor` _asbp_carne_cruda)
      (bind _returnvalue (`|SpawnActorFromClass` "/Game/Blueprints/BP_Carne_Cocida.BP_Carne_Cocida_C" (`SceneComponent.K2_GetComponentToWorld` (`self.PuntoDeEntrega`)) "Undefined" "MultiplyWithRoot" null null))
      (set `self.CarneEnHorno` _returnvalue))))

(fn `UserConstructionScript`
  (`parent.UserConstructionScript`))