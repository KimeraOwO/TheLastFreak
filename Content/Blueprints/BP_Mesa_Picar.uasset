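; BP_Mesa_Picar is an interactable chopping table that turns the object held by a BP_Cuidador into chopped tomato.
; Interactuar calls its parent, waits on a fixed delay, then casts the interactor.
; With no stored product, it destroys the held object without checking its type and spawns BP_Tomate_Picado at PuntoDeEntrega, storing it as ProductoProcesado.
; Otherwise, it forwards the interaction to that product and clears the reference.
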(event `/Game/Blueprints/BPI_Interaccion.Interactuar`
  (params (Interactor :type "Actor Object Reference"))
  (bind _productoprocesado (`self.ProductoProcesado`))
  (`parent.Interactuar` (stale _asbp_cuidador))
  (`KismetSystemLibrary.Delay` 3.0)
  (bind _asbp_cuidador (cast `/Game/Blueprints/BP_Cuidador` Interactor))
  (`/Engine/EditorBlueprintResources/StandardMacros.IsValid` _productoprocesado
    (:`Is Valid`
      (message `/Game/Blueprints/BPI_Interaccion.Interactuar` _productoprocesado _asbp_cuidador)
      (set `self.ProductoProcesado` null))
    (:`Is Not Valid`
      (`self.K2_DestroyActor` (`/Game/Blueprints/BP_Cuidador.ObjetoAgarrado` _asbp_cuidador))
      (bind _returnvalue (`|SpawnActorFromClass` "/Game/Blueprints/BP_Tomate_Picado.BP_Tomate_Picado_C" (`SceneComponent.K2_GetComponentToWorld` (`self.PuntoDeEntrega`)) "Undefined" "MultiplyWithRoot" null null))
      (set `self.ProductoProcesado` _returnvalue))))

(fn `UserConstructionScript`
  (`parent.UserConstructionScript`))