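; BP_Mesa_Preparacion is a preparation table where a BP_Cuidador assembles tacos from held ingredients.
; Interactuar calls its parent, then casts the held object to tortilla, cooked meat or chopped tomato, flags that ingredient and destroys the item.
; Once all three flags are set, it spawns a BP_Taco at PuntoDeEntrega.
; The graph never resets the flags, so each later valid ingredient spawns another taco.
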(event `/Game/Blueprints/BPI_Interaccion.Interactuar`
  (params (Interactor :type "Actor Object Reference"))
  (`parent.Interactuar` (stale _asbp_cuidador))
  (bind _asbp_cuidador (cast `/Game/Blueprints/BP_Cuidador` Interactor))
  (bind _objetoagarrado (`/Game/Blueprints/BP_Cuidador.ObjetoAgarrado` _asbp_cuidador))
  (bind _asbp_tortilla (cast `/Game/Blueprints/BP_Tortilla` _objetoagarrado)
    (:`then`
      (bind _output_get (set `self.TieneTortilla` true))
      (`self.K2_DestroyActor` _asbp_tortilla))
    (:`CastFailed`
      (bind _asbp_carne_cocida (cast `/Game/Blueprints/BP_Carne_Cocida` _objetoagarrado)
        (:`then`
          (bind _output_get_2 (set `self.TieneCarne` true))
          (`self.K2_DestroyActor` _asbp_carne_cocida))
        (:`CastFailed`
          (bind _asbp_tomate_picado (cast `/Game/Blueprints/BP_Tomate_Picado` _objetoagarrado))
          (bind _output_get_3 (set `self.TieneTomate` true))
          (`self.K2_DestroyActor` _asbp_tomate_picado)))))
  (if (and _output_get _output_get_2 _output_get_3)
    (`|SpawnActorFromClass` "/Game/Blueprints/BP_Taco.BP_Taco_C" (`SceneComponent.K2_GetComponentToWorld` (`self.PuntoDeEntrega`)) "Undefined" "MultiplyWithRoot" null null)))

(fn `UserConstructionScript`
  (`parent.UserConstructionScript`))