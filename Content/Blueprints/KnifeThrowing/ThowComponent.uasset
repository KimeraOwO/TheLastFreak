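; Knife-throwing component for the BP_Cuidador player that caches its owner on BeginPlay.
; Shoot spawns a ThrowableKnifes actor at the owner's root location, facing the controller's aim direction.
; It then applies an impulse to the knife's Sphere, scaled from the new actor's current velocity rather than from the aim vector.
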(event `self.ReceiveBeginPlay`
  (bind _asbp_cuidador (cast `/Game/Blueprints/BP_Cuidador` (`self.GetOwner`)))
  (set `self.As BP Cuidador` _asbp_cuidador))

(event `Shoot`
  (bind _as_bp_cuidador (`self.As BP Cuidador`))
  (bind _returnvalue (`|SpawnActorFromClass` "/Game/Blueprints/KnifeThrowing/ThrowableKnifes.ThrowableKnifes_C" (`KismetMathLibrary.MakeTransform` (`SceneComponent.K2_GetComponentLocation` (`Actor.RootComponent` _as_bp_cuidador)) (`KismetMathLibrary.Conv_VectorToRotator` (`KismetMathLibrary.GetForwardVector` (`Controller.GetControlRotation` (`Pawn.GetController` _as_bp_cuidador))))) "Undefined" "MultiplyWithRoot" null null))
  (`PrimitiveComponent.AddImpulse` (`/Game/Blueprints/KnifeThrowing/ThrowableKnifes.Sphere` _returnvalue) (* (`Actor.GetVelocity` _returnvalue) 100.0) "None" false))