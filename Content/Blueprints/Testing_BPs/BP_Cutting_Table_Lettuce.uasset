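; Cutting table station that turns its current ingredient into chopped lettuce.
; StartProcessing waits out a delay, destroys the current ingredient, then spawns BP_Lettuce_Chopped at the placement point as the new current ingredient, marked Processed.
; It then clears the processing flag and plays the station VFX for a few seconds.
; The output class is hardcoded, with no check on the ingredient type in this graph.
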(event `self.StartProcessing`
  (bind _stationvfx (`self.StationVFX`))
  (`KismetSystemLibrary.Delay` 3.0)
  (`self.K2_DestroyActor` (`self.CurrentIngredient`))
  (bind _returnvalue (`|SpawnActorFromClass` "/Game/Blueprints/BP_Lettuce_Chopped.BP_Lettuce_Chopped_C" (`SceneComponent.K2_GetComponentToWorld` (`self.ItemPlacementPoint`)) "AlwaysSpawn" "MultiplyWithRoot" null null))
  (bind _output_get (set `self.CurrentIngredient` _returnvalue))
  (`Ingredient.SetIngredientState` _output_get "Processed")
  (`self.SetProcessingFalse`)
  (`ActorComponent.Activate` _stationvfx true)
  (`KismetSystemLibrary.Delay` 3.0)
  (`ActorComponent.Deactivate` _stationvfx))

(fn `UserConstructionScript`)